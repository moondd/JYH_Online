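; Base character Blueprint for networked action combat with combo attacks, skills, dodge, jump and hit knockback.
; Base, action and in-air states, changed mainly on authority, gate input and drive montages, eased mesh-only rotation and energy recovery.
; Attacks read DT_SkillData; anim-notify damage sphere-overlaps pawns, filters by angle and height, spends energy and triggers montage hit-stop.
; Point damage enters the hit state and runs timeline-driven knockback with hit effects.
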(event `CE_UpdateCharacterRotation`
  (bind _returnvalue (`self.GetVelocity`))
  (bind _pre_characterrotation (`self.Pre_CharacterRotation`))
  (bind _returnvalue_2 (> (`KismetMathLibrary.VSizeXY` _returnvalue) 100.0))
  (`|ExecutionSequence` :!label _label
    (:`then_0`
      (switch `/Game/GameData/E_CharacterState_Base` (`self.CharacterState_Base`)
        (:`NewEnumerator0`
          (switch `/Game/GameData/E_CharacterState_Action` (`self.CharacterState_Action`)
            (:`NewEnumerator0`
              (if _returnvalue_2
                (set `self.Sev_CharacterRotation` (`KismetMathLibrary.SelectRotator` (`KismetMathLibrary.Conv_VectorToRotator` _returnvalue) _pre_characterrotation _returnvalue_2))
                (`self.SetCharacterRotation` (`self.Sev_CharacterRotation`) :!label _label_2)
                (set `self.Pre_CharacterRotation` (`KismetMathLibrary.MakeRotator` 0.0 0.0 (+ (.yaw (`SceneComponent.K2_GetComponentRotation` (`self.Mesh`))) 90.0)))))
            (:`NewEnumerator2`
              (set `self.Sev_CharacterRotation` (`self.CurrInputRotation`) :!label _label_3)
              (goto _label_2))
            (:`NewEnumerator3`
              (set `self.Sev_CharacterRotation` _pre_characterrotation :!label _label_4)
              (goto _label_2))
            (:`NewEnumerator4`
              (goto _label_3))))
        (:`NewEnumerator1`
          (goto _label_4))))))

(event `self.ReceiveBeginPlay`
  (bind _asbp_character_anim (cast `/Game/Blueprint/Character/BP_Character_Anim` (`SkeletalMeshComponent.GetAnimInstance` (`self.Mesh`))))
  (set `self.AnimInstance` _asbp_character_anim))

(event `CE_Loc_UpdateCharacterRotation`
  (goto _label))

(event `self.ReceiveTick`
  (params (DeltaSeconds :type "Float (single-precision)"))
  (if (`KismetSystemLibrary.IsDedicatedServer`)
    (`/Engine/EditorBlueprintResources/ActorMacros.Switch Has Authority`
      (:`Authority`
        (`self.CE_UpdateCharacterRotation`)
        (`self.RecoverEnergy`))
      (:`Remote`
        (`self.CE_RotatCharacter`)))
    (else
      (`self.CE_Loc_UpdateCharacterRotation`)
      (`self.RecoverEnergy`))))

(event `CE_RotatCharacter`
  (`self.SetCharacterRotation` (`self.Sev_CharacterRotation`)))

(event `CE_Attack_Server`
  (`self.CE_Action_Attack_Input_Svr`))

(event `CE_CurrEnergyChanged`)

(event `CE_ChangeCharacterState_Action_Sev`
  (params (CharacterStateAction :type "/Game/GameData/E_CharacterState_Action Enum" :default "NewEnumerator0"))
  ;[1 1 1] 地面行为
  (`self.CE_EnterCharacterState_Action` (`self.CharacterState_Action`) CharacterStateAction)
  (set `self.CharacterState_Action` CharacterStateAction))

(event `CE_ChangeCharacterState_InAir_Sev`
  (params (CharacterStateInAir :type "/Game/GameData/E_CharacterState_InAir Enum" :default "NewEnumerator0"))
  ;[1 1 1] 空中行为
  (`self.CE_EnterCharacterState_InAir` (`self.CharacterState_InAir`) CharacterStateInAir))

(event `self.K2_OnMovementModeChanged`
  (params (PrevMovementMode :type "EMovementMode Enum" :default "MOVE_None") (NewMovementMode :type "EMovementMode Enum" :default "MOVE_None") (PrevCustomMode :type Byte) (NewCustomMode :type Byte))
  ;[1 1 1] MoveMode
  (if (`KismetSystemLibrary.IsDedicatedServer`)
    (`/Engine/EditorBlueprintResources/ActorMacros.Switch Has Authority`
      (:`Authority`
        _)))
  (`|ExecutionSequence`
    (:`then_0`
      (switch `EMovementMode` PrevMovementMode
        (:`MOVE_Falling`
          (`self.CE_ChangeCharacterState_Action_Sev` "NewEnumerator0")
          (`self.CE_ChangeCharacterState_InAir_Sev` "NewEnumerator0"))))
    (:`then_1`
      (switch `EMovementMode` NewMovementMode))))

(event `CE_ChangeCharacterState_Base_Sev`
  (params (CharacterStateBase :type "/Game/GameData/E_CharacterState_Base Enum" :default "NewEnumerator0"))
  ;[1 1 1] 主状态
  (`self.CE_EnterCharacterStateBase` (`self.CharacterState_Base`) CharacterStateBase)
  (set `self.CharacterState_Base` CharacterStateBase))

(event `CE_EnterCharacterStateBase`
  (params (Leave :type "/Game/GameData/E_CharacterState_Base Enum" :default "NewEnumerator0") (Enter :type "/Game/GameData/E_CharacterState_Base Enum" :default "NewEnumerator0"))
  ;[1 1 1] 主状态
  (`|ExecutionSequence`
    (:`then_0`
      (switch `/Game/GameData/E_CharacterState_Base` Leave))
    (:`then_1`
      (switch `/Game/GameData/E_CharacterState_Base` Enter
        (:`NewEnumerator1`
          (`/Engine/EditorBlueprintResources/ActorMacros.Switch Has Authority`
            (:`Authority`
              (`self.CE_ChangeCharacterState_Action_Sev` "NewEnumerator0"))))))))

(event `CE_EnterCharacterState_InAir`
  (params (Leave :type "/Game/GameData/E_CharacterState_InAir Enum" :default "NewEnumerator0") (Enter :type "/Game/GameData/E_CharacterState_InAir Enum" :default "NewEnumerator0"))
  ;[1 1 1] 空中行为
  (`|ExecutionSequence`
    (:`then_0`
      (switch `/Game/GameData/E_CharacterState_InAir` Leave))
    (:`then_1`
      (switch `/Game/GameData/E_CharacterState_InAir` Enter
        (:`NewEnumerator1`
          (`AnimInstance.Montage_Stop` (`self.AnimInstance`) 0.1 null)
          (`self.Jump`))))))

(event `CE_EnterCharacterState_Action`
  (params (Leave :type "/Game/GameData/E_CharacterState_Action Enum" :default "NewEnumerator0") (Enter :type "/Game/GameData/E_CharacterState_Action Enum" :default "NewEnumerator0"))
  ;[1 1 1] 地面行为
  (`|ExecutionSequence`
    (:`then_0`
      (switch `/Game/GameData/E_CharacterState_Action` Leave
        (:`NewEnumerator2`
          (`MovementComponent.SetPlaneConstraintNormal` (`self.CharacterMovement`) (0.0 0.0 0.0))
          (`/Engine/EditorBlueprintResources/ActorMacros.Switch Has Authority`
            (:`Authority`
              (if (`|EnumInequality` Enter "NewEnumerator3")
                (`self.CE_Action_Attack_End_Svr` :!label _label)))))
        (:`NewEnumerator3`
          (`/Engine/EditorBlueprintResources/ActorMacros.Switch Has Authority`
            (:`Authority`
              (if (`|EnumInequality` Enter "NewEnumerator2")
                (goto _label)))))))
    (:`then_1`
      (switch `/Game/GameData/E_CharacterState_Action` Enter
        (:`NewEnumerator2`
          (`/Engine/EditorBlueprintResources/ActorMacros.Switch Has Authority`
            (:`Authority`
              (`self.UpdateCurrInputRotation`)
              (set `self.Sev_CharacterRotation` (`self.CurrInputRotation`))
              (set `self.CurrAttackTime` 0.0)
              (set `self.CurrSkillDamageNumber` 0)
              (`self.CE_PlayAttackAnimation_Multi` (`|GetArrayItem` (`self.CurrGestArray`))))))
        (:`NewEnumerator3`
          (`/Engine/EditorBlueprintResources/ActorMacros.Switch Has Authority`
            (:`Authority`
              (set `self.CurrAttackTime` 0.0))))
        (:`NewEnumerator4`
          (`/Engine/EditorBlueprintResources/ActorMacros.Switch Has Authority`
            (:`Authority`
              (`self.UpdateCurrInputRotation`)
              (set `self.Sev_CharacterRotation` (`self.CurrInputRotation`))
              (`self.CE_Action_Dodge_Multi`))))))))

(event `CE_Action_Attack_Input_Svr`
  ;[1 1 1] 攻击
  (if (not (> (`KismetArrayLibrary.Array_Length` (`self.CurrGestArray`)) 0))
    (set `self.CurrGestArray` (`self.GestArray_Normal`)))
  (`self.CE_Action_Attack_Skill_Svr` (`|GetArrayItem` (`self.CurrGestArray`))))

(event `CE_Damage_AnimNotify_Svr`
  ;[1 1 1] 造成伤害
  (`self.CE_Damage_New_Svr`)
  (`/Engine/EditorBlueprintResources/StandardMacros.IncrementInt` (`self.CurrSkillDamageNumber`)
    (:`  `
      (`|ExecutionSequence`
        (:`then_0`
          ;[1 1 1] 攻击消耗
          (set `self.CurrEnergy` (- (`self.CurrEnergy`) (* (`self.CurrAttackTime`) 70.0)))
          (`self.CE_CurrEnergyChanged`))
        (:`then_1`
          (set `self.CurrAttackTime` 0.0))))))

(event `CE_Action_Attack_Skill_Svr`
  (params (GestName :type Name))
  (bind _currgestarray (`self.CurrGestArray`))
  ;[1 1 1] 攻击
  (bind (_can _maneconsume _skilltype) (`self.CanUseSkill` GestName))
  (if _can
    (switch `/Game/GameData/E_GestType` _skilltype
      (:`NewEnumerator0`
        _)
      (:`NewEnumerator1`
        (`KismetArrayLibrary.Array_Clear` _currgestarray)
        (`KismetArrayLibrary.Array_Add` _currgestarray GestName)
        (`self.ManaConsume` _maneconsume)))
    (`self.CE_ChangeCharacterState_Action_Sev` "NewEnumerator2")))

(event `CE_Damage_New_Svr`
  ;[1 1 1] 造成伤害
  (bind (_outdamagetargetarray _outdamagedata) (`self.FindDamageTarget`))
  (`|ExecutionSequence`
    (:`then_0`
      (for _array_element _outdamagetargetarray
        (bind _asbp_character_base (cast `/Game/Blueprint/Character/BP_Character_Base` _array_element))
        (`GameplayStatics.ApplyPointDamage` _asbp_character_base 10.0 (`KismetMathLibrary.GreaterGreater_VectorRotator` (`SceneComponent.GetRightVector` (`self.Mesh`)) (`KismetMathLibrary.MakeRotator` 0.0 0.0 (`.DamageRotAdd_3_370771334234756FD9BEBAA0F74A2DC4` (break `/Game/GameData/S_DamageData` _outdamagedata)))) (`GameplayStatics.MakeHitResult` false) null self)))
    (:`then_1`
      (if (> (`KismetArrayLibrary.Array_Length` _outdamagetargetarray) 0)
        (`self.DoDamageEffect`)))))

(event `CE_Action_Attack_End_Svr`
  ;[1 1 1] 攻击
  ;;[1 1 1] 攻击结束
  (`KismetArrayLibrary.Array_Clear` (`self.CurrGestArray`))
  (set `self.CurrSkillDamageNumber` 0))

(event `DoDamageEffect`
  (bind _animinstance (`self.AnimInstance`))
  (bind _returnvalue (`AnimInstance.GetCurrentActiveMontage` _animinstance))
  (`AnimInstance.Montage_SetPlayRate` _animinstance _returnvalue 0.1)
  (`KismetSystemLibrary.Delay` 0.1)
  (`AnimInstance.Montage_SetPlayRate` _animinstance _returnvalue 1.0))

(event `CE_Action_Attack_Combo_Svr`
  ;[1 1 1] 攻击
  ;;[1 1 1] 连击通知
  (`self.CE_ChangeCharacterState_Action_Sev` "NewEnumerator3"))

(event `self.ReceivePointDamage`
  (params (Damage :type "Float (single-precision)") (DamageType :type "DamageType Object Reference") (HitLocation :type "Vector Structure") (HitNormal :type "Vector Structure") (HitComponent :type "PrimitiveComponent Object Reference") (BoneName :type Name) (ShotFromDirection :type "Vector Structure") (InstigatedBy :type "Controller Object Reference") (DamageCauser :type "Actor Object Reference") (HitInfo :type "HitResult Structure (by ref)"))
  (bind (_returnvalue_roll _returnvalue_pitch _returnvalue_yaw) (`KismetMathLibrary.BreakRotator` (`KismetMathLibrary.NormalizedDeltaRotator` (`KismetMathLibrary.MakeRotFromX` (`SceneComponent.GetRightVector` (`self.Mesh`))) (`KismetMathLibrary.Conv_VectorToRotator` ShotFromDirection))))
  (`self.CE_ChangeCharacterState_Base_Sev` "NewEnumerator1")
  (`self.CE_Action_Blow_Multi` ShotFromDirection _returnvalue_yaw 650.0))

(event `CE_PlayAttackAnimation_Multi`
  (params (GestName :type Name))
  ;[1 1 1] 攻击
  ;;[1 1 1] 同步播放动画
  (`self.PlayAttackAnimation` GestName
    (:`Then`
      (`/Engine/EditorBlueprintResources/ActorMacros.Switch Has Authority`
        (:`Authority`
          (`KismetArrayLibrary.Array_Remove` (`self.CurrGestArray`)))))
    (:`Completed`
      (`/Engine/EditorBlueprintResources/ActorMacros.Switch Has Authority`
        (:`Authority`
          (`self.CE_ChangeCharacterState_Action_Sev` "NewEnumerator0"))))))

(event `Event_TrailBegin`
  ;[1 1 1] 攻击
  ;;[1 1 1] 攻击特效
)

(event `Event_TrailEnd`
  ;[1 1 1] 攻击
  ;;[1 1 1] 攻击特效
)

(event `CE_Action_Blow_Multi`
  (params (BlowVector :type "Vector Structure") (BeDamageRot :type "Float (double-precision)") (ForceAdd :type "Float (double-precision)" :default 1.0) (StartTime :type "Float (double-precision)" :default 0.0))
  (bind _charactermovement (`self.CharacterMovement`))
  (bind _animinstance (`self.AnimInstance`))
  (bind (_returnvalue_location _returnvalue_rotation) (`KismetMathLibrary.BreakTransform` (`SceneComponent.GetSocketTransform` (`self.Mesh`) "Bip001-Spine2" "RTS_World")))
  (`AnimInstance.Montage_Stop` _animinstance 0.1 null)
  (if (`KismetSystemLibrary.IsDedicatedServer`)
    (`/Engine/EditorBlueprintResources/ActorMacros.Switch Has Authority`
      (:`Authority`
        (`|ExecutionSequence` :!label _label
          (:`then_0`
            (bind (_direction _float) (`Timeline|BlowTime` :`NewTime` StartTime :!via `SetNewTime` :!label _label_2)
              (:`Finished`
                (`/Engine/EditorBlueprintResources/ActorMacros.Switch Has Authority`
                  (:`Authority`
                    (`self.CE_ChangeCharacterState_Base_Sev` "NewEnumerator0"))))))
          (:`then_1`
            (goto _label_2 :!via `PlayFromStart`))
          (:`then_2`
            (set `MovementComponent.Velocity` (`KismetMathLibrary.MakeVector` (.x (* BlowVector (* ForceAdd _float))) (.y (* BlowVector (* ForceAdd _float))) (.z (`MovementComponent.Velocity` _charactermovement))) _charactermovement))))
      (:`Remote`
        (`/Game/Blueprint/Character/BP_Character_Anim.CE_NewDamaged` _animinstance BeDamageRot :!label _label_3)
        (`|ExecutionSequence`
          (:`then_0`
            ;[1 1 1] 受击特效
            (`GameplayStatics.SpawnEmitterAtLocation` "/Game/Res/Effect/Damage/BeDamage_Normal.BeDamage_Normal" _returnvalue_location _returnvalue_rotation))
          (:`then_1`
            (goto _label)))))
    (else
      (goto _label_3))))

(event `CE_Action_Jump_Svr`
  (if (`self.CanJump?`)
    (`self.CE_ChangeCharacterState_InAir_Sev` "NewEnumerator1")))

(event `CE_Action_Dodge_Svr`
  (if (`self.CanAttack?`)
    (`self.CE_ChangeCharacterState_Action_Sev` "NewEnumerator4")))

(event `CE_Action_Dodge_Multi`
  (`|PlayMontage` (`self.Mesh`) "/Game/Res/Character/Anim/Dodge/Anim_Dodge_F_Montage.Anim_Dodge_F_Montage" 1.0 0.0 "Start"
    (:`OnBlendOut`
      (`/Engine/EditorBlueprintResources/ActorMacros.Switch Has Authority`
        (:`Authority`
          (`self.CE_ChangeCharacterState_Action_Sev` "NewEnumerator0"))))))

(fn `CanAttack?`
  (returns (`Can?` :type Boolean))
  (if (> (`self.CurrEnergy`) 0.0)
    (`|ExecutionSequence`
      (:`then_0`
        (switch `EMovementMode` (`CharacterMovementComponent.MovementMode` (`self.CharacterMovement`))
          (:`MOVE_Walking`
            (switch `/Game/GameData/E_CharacterState_Base` (`self.CharacterState_Base`)
              (:`NewEnumerator0`
                (switch `/Game/GameData/E_CharacterState_Action` (`self.CharacterState_Action`)
                  (:`NewEnumerator0`
                    _)
                  (:`NewEnumerator1`
                    _)
                  (:`NewEnumerator3`
                    _))
                (return true))))))
      (:`then_1`
        _)))
  (return false))

(fn `CanJump?`
  (returns (`Can?` :type Boolean))
  (if (`self.CanJump`)
    (`|ExecutionSequence`
      (:`then_0`
        (switch `EMovementMode` (`CharacterMovementComponent.MovementMode` (`self.CharacterMovement`))
          (:`MOVE_Walking`
            (switch `/Game/GameData/E_CharacterState_Base` (`self.CharacterState_Base`)
              (:`NewEnumerator0`
                (switch `/Game/GameData/E_CharacterState_Action` (`self.CharacterState_Action`)
                  (:`NewEnumerator0`
                    _)
                  (:`NewEnumerator1`
                    _)
                  (:`NewEnumerator3`
                    _))
                (return true))))))
      (:`then_1`
        _)))
  (return false))

(fn `CanMove?`
  (returns (`Can?` :type Boolean))
  (`|ExecutionSequence`
    (:`then_0`
      (switch `EMovementMode` (`CharacterMovementComponent.MovementMode` (`self.CharacterMovement`))
        (:`MOVE_Walking`
          _)
        (:`MOVE_NavWalking`
          _))
      (switch `/Game/GameData/E_CharacterState_Base` (`self.CharacterState_Base`)
        (:`NewEnumerator0`
          (switch `/Game/GameData/E_CharacterState_Action` (`self.CharacterState_Action`)
            (:`NewEnumerator0`
              _)
            (:`NewEnumerator1`
              _))
          (return true))))
    (:`then_1`
      (return false))))

(fn `CanUseSkill`
  (params (InSkillName :type Name))
  (returns (Can :type Boolean) (ManeConsume :type "Float (double-precision)") (SkillType :type "/Game/GameData/E_GestType Enum"))
  (if (`self.IsCombat?`)
    (if (`self.CanAttack?`)
      (bind _returnvalue (`|GetDataTableRow` "/Game/GameData/DT_SkillData.DT_SkillData" InSkillName)
        (:`then`
          (bind (_name _gesttype _weapontype _anim_m) (break `/Game/GameData/S_SkillData` _returnvalue))
          (switch `/Game/GameData/E_GestType` _gesttype
            (:`NewEnumerator0`
              (return true 0.0 "NewEnumerator0"))
            (:`NewEnumerator1`
              (bind _returnvalue_2 (* (`AnimSequenceBase.SequenceLength` _anim_m) 30.0))
              (return (>= (`self.CurrMana`) _returnvalue_2) _returnvalue_2 _gesttype))))
        (:`RowNotFound`
          _))))
  (return false 0.0 "NewEnumerator0"))

(fn `FindDamageTarget`
  (returns (OutDamageTargetArray :type "Array of Actor Object Reference") (OutDamageData :type "/Game/GameData/S_DamageData Structure"))
  (locals (Loc_DamageTargets :type "Array of Actor Object Reference"))
  (bind _returnvalue (`SceneComponent.K2_GetComponentLocation` (`self.Mesh`)))
  (bind _output (`|GetArrayItem` (`.DamageDataArray_26_A5FE441848387189463D16B0486C7F47` (break `/Game/GameData/S_SkillData` (`self.CurrSkillData`))) (`self.CurrSkillDamageNumber`)))
  (bind (_damagerotadd _damageaddition _distence _angle _max_z _min_z) (break `/Game/GameData/S_DamageData` _output))
  (bind _outactors (`KismetSystemLibrary.SphereOverlapActors` (`SceneComponent.GetSocketLocation` (`self.Mesh`) "Bip001") _distence (`|MakeArray` "ObjectTypeQuery3" :!type "EObjectTypeQuery Enum") null (`|MakeArray` self :!type "Actor Object Reference")))
  (for _array_element _outactors
    (bind _asbp_character_base (cast `/Game/Blueprint/Character/BP_Character_Base` _array_element))
    (bind _returnvalue_2 (`SceneComponent.K2_GetComponentLocation` (`Character.Mesh` _asbp_character_base)))
    (bind (_returnvalue_roll _returnvalue_pitch _returnvalue_yaw) (`KismetMathLibrary.BreakRotator` (`KismetMathLibrary.NormalizedDeltaRotator` (`KismetMathLibrary.FindLookAtRotation` _returnvalue _returnvalue_2) (`KismetMathLibrary.Conv_VectorToRotator` (`SceneComponent.GetRightVector` (`self.Mesh`))))))
    (if (and (`KismetMathLibrary.InRange_FloatFloat` (`KismetMathLibrary.Abs` _returnvalue_yaw) 0.0 _angle) (`KismetMathLibrary.InRange_FloatFloat` (- (.z _returnvalue_2) (.z _returnvalue)) _min_z _max_z))
      (`KismetArrayLibrary.Array_Add` (`local.Loc_DamageTargets`) _array_element)))
  (return (`local.Loc_DamageTargets`) _output))

(fn `ManaConsume`
  (params (Consume :type "Float (double-precision)"))
  (set `self.CurrMana` (- (`self.CurrMana`) Consume)))

(fn `OnRep_IsCombat?`)

(fn `OnRep_SaveVector`)

(fn `SetCharacterRotation`
  (params (InRot :type "Rotator Structure"))
  (bind (_result_roll _result_pitch _result_yaw) (`KismetMathLibrary.BreakRotator` (`|EaseFunction` "SinusoidalInOut" 0.25 (`self.Pre_CharacterRotation`) InRot)))
  (`|ExecutionSequence`
    (:`then_0`
      (`SceneComponent.K2_SetWorldRotation` (`self.Mesh`) (`KismetMathLibrary.MakeRotator` 0.0 0.0 (- _result_yaw 90.0)) false false)
      (switch `/Game/GameData/E_CharacterState_Action` (`self.CharacterState_Action`)
        (:`NewEnumerator2`
          (`MovementComponent.SetPlaneConstraintNormal` (`self.CharacterMovement`) (`SceneComponent.GetForwardVector` (`self.Mesh`))))))
    (:`then_1`
      (return))))

(fn `UpdateCurrInputRotation`
  (bind _returnvalue (`KismetMathLibrary.MakeRotator` 0.0 0.0 (.yaw (`self.GetControlRotation`))))
  (bind _returnvalue_2 (+ (* (`KismetMathLibrary.GetForwardVector` _returnvalue) (`self.Input_Y`)) (* (`KismetMathLibrary.GetRightVector` _returnvalue) (`self.Input_X`))))
  (set `self.CurrInputRotation` (`KismetMathLibrary.SelectRotator` (`KismetMathLibrary.Conv_VectorToRotator` _returnvalue_2) (`self.Pre_CharacterRotation`) (!= _returnvalue_2 (0.0 0.0 0.0))))
  (return))

(fn `UserConstructionScript`)
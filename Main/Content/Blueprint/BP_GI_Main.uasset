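; Game instance Blueprint that opens the multiplayer session menus and launches hosted games.
; Custom events lazily create, cache and display the search-games and host-game widgets.
; The lobby launch event stores the server name and creates a session, using LAN when Steam is not selected.
; On success it opens ThirdPersonExampleMap as a listen server, and on failure it prints an error.
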(event `CE_SearchGameMenu`
  (`/Engine/EditorBlueprintResources/StandardMacros.IsValid` (`self.SearchGames`)
    (:`Is Valid`
      _)
    (:`Is Not Valid`
      (bind _returnvalue (`|CreateWidget` "/Game/UI/W_SearchGames.W_SearchGames_C" (`GameplayStatics.GetPlayerController` 0)))
      (set `self.SearchGames` _returnvalue)))
  (`UserWidget.AddToViewport` (`self.SearchGames`) 0))

(event `CE_HostGameMenu`
  (`/Engine/EditorBlueprintResources/StandardMacros.IsValid` (`self.HostGame`)
    (:`Is Valid`
      _)
    (:`Is Not Valid`
      (bind _returnvalue (`|CreateWidget` "/Game/UI/W_HostGame.W_HostGame_C" (`GameplayStatics.GetPlayerController` 0)))
      (set `self.HostGame` _returnvalue)))
  (`UserWidget.AddToViewport` (`self.HostGame`) 0))

(event `CE_LaunchLobby`
  (params (`IsSteam?` :type Boolean) (ServerName :type Text))
  (set `self.ServerName` ServerName)
  (`CreateSessionCallbackProxy.CreateSession` (`GameplayStatics.GetPlayerController` 0) 20 (not `IsSteam?`)
    (:`OnSuccess`
      (`GameplayStatics.OpenLevel` "ThirdPersonExampleMap" true "listen"))
    (:`OnFailure`
      (`KismetSystemLibrary.PrintString` "CreatLobbyFailed"))))